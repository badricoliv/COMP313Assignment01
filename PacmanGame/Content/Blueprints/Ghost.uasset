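; Ghost actor that wanders along the X and Y axes, changing course whenever it hits something.
; A looping timer started at BeginPlay calls rollMovement, which applies a swept world offset using the stored Location vector as a per-tick step.
; Each Hit event flips the Direction toggle to alternate between axes and randomly picks the positive or negative way along the new axis.
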(event Custom|rollMovement
  (Transformation|AddActorWorldOffset (Variables|Default|GetLocation) true))

(event Collision|EventHit
  (params (MyComp :type Primitive%20Component%20Object%20Reference) (Other :type Actor%20Object%20Reference) (OtherComp :type Primitive%20Component%20Object%20Reference) (bSelfMoved :type Boolean) (HitLocation :type Vector :default "0, 0, 0") (HitNormal :type Vector :default "0, 0, 0") (NormalImpulse :type Vector :default "0, 0, 0") (Hit :type Hit%20Result%20Structure%20%28by%20ref%29))
  (if (== (Variables|Default|Getdirection) 0)
    (if (Math|Random|RandomBool)
      (Variables|Default|SetLocation "-2.500000, 0, 0")
      (else
        (Variables|Default|SetLocation "2.500000, 0, 0")))
    (Variables|Default|Setdirection 1)
    (else
      (if (Math|Random|RandomBool)
        (Variables|Default|SetLocation "0.000000,-2.500000, 0")
        (else
          (Variables|Default|SetLocation "0.000000,2.500000, 0")))
      (Variables|Default|Setdirection 0))))

(event EventBeginPlay
  (Utilities|Time|SetTimerbyFunctionName 0 "rollMovement" 0.008 true))

(fn ConstructionScript)